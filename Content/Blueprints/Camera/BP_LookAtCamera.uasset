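; BP_LookAtCamera is a camera actor that keeps its view turned toward the player.
; On BeginPlay it stores the first player pawn as its target.
; Every tick it sets the camera component's world rotation with FindLookAtRotation toward that target, then calls UpdateCameraDistance, which is currently an empty stub.
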(event Custom|UpdateCameraLookat
  (bind _cameracomponent (Variables|CameraActor|GetCameraComponent))
  ;[1 1 1] Track Player With Camera
  (Transformation|SetWorldRotation _cameracomponent (Math|Rotator|FindLookatRotation (Transformation|GetWorldLocation _cameracomponent) (Transformation|GetActorLocation (Variables|Default|GetTargetActor))) false false))

(event EventBeginPlay
  ;[1 1 1] Set Camera Rotation To Player At Start
  (Variables|Default|SetTargetActor (Game|Player|GetPlayerPawn 0)))

(event Collision|EventActorBeginOverlap
  (params (OtherActor :type Actor%20Object%20Reference)))

(event EventTick
  (params (DeltaSeconds :type Float%20%28single-precision%29))
  ;[1 1 1] Constantly Check And Update Camera Rotation / Note: Optomoize By Finding Better Option Than Event Tick
  (CallFunction|UpdateCameraLookat)
  (CallFunction|UpdateCameraDistance))

(fn ConstructionScript)

(fn UpdateCameraDistance)